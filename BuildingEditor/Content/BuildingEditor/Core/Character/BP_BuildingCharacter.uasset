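; Player character for the building editor, handling camera movement, turning, zooming and a grid-snapped wall cursor.
; Enhanced Input actions feed movement, turn and zoom functions, with a timeline adding inertia to zoom.
; Tick traces under the mouse and snaps WallCursor to the grid.
; A custom cursor widget replaces the system cursor and changes icon while rotate or translate toggles are active.
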(event EventBeginPlay
  (Input|AddMappingContext (PlayerController|LocalPlayerSubsystems|GetEnhancedInputLocalPlayerSubsystem (Game|GetPlayerController 0)) "/Game/BuildingEditor/Core/Inputs/IMC_BuildingEditor.IMC_BuildingEditor" 0 "(bIgnoreAllPressedKeysUntilRelease=True,bForceImmediately=False,bNotifyUserSettings=False)")
  (Components|Timeline|SetPlayRate (Variables|Default|GetScrollTimeline) (/ 1.0 (Variables|Default|GetScrollInertia)))
  (bind _returnvalue (UserInterface|CreateWidget "/Game/BuildingEditor/Core/Character/Widgets/WBP_Cursor.WBP_Cursor_C" 0 (Variables|BuildingPawn|CursorIcons|GetDefaultCursor)))
  (Variables|Default|SetCursorWidget _returnvalue)
  (bind _asplayer_controller (Utilities|Casting|CastToPlayerController (Pawn|GetController)))
  (bind _output_get (Variables|Default|SetPlayerController _asplayer_controller))
  (Class|PlayerController|SetMouseCursorWidget _output_get "Default" (Variables|Default|GetCursorWidget))
  (Variables|/Script/Engine.PlayerController|SetbShowMouseCursor (Variables|Default|GetPlayerController) false))

(event EventTick
  (params (DeltaSeconds :type Float%20%28single-precision%29))
  (Transformation|SetWorldLocation (Variables|Default|GetWallCursor) (CallFunction|SnaptoGrid (.Location (Collision|BreakHitResult (.HitResult (Game|Player|GetHitResultUnderCursorbyChannel (Variables|Default|GetPlayerController) "TraceTypeQuery1" true)))) 100) false false))

(event Input|EnhancedActionEvents|EnhancedInputActionIA_Movement
  (params (ActionValue :type Vector%202D%20Structure) (ElapsedSeconds :type Float%20%28double-precision%29) (TriggeredSeconds :type Float%20%28double-precision%29) (InputAction :type Input%20Action%20Object%20Reference :default "/Game/BuildingEditor/Core/Inputs/IA/IA_Movement.IA_Movement"))
  (bind (_x _y) (Math|Vector2D|BreakVector2D ActionValue))
  (Class|BuildingPawn|MoveForward _x)
  (Class|BuildingPawn|MoveRight _y))

(event Input|EnhancedActionEvents|EnhancedInputActionIA_Turn
  (params (ActionValue :type Float%20%28double-precision%29) (ElapsedSeconds :type Float%20%28double-precision%29) (TriggeredSeconds :type Float%20%28double-precision%29) (InputAction :type Input%20Action%20Object%20Reference :default "/Game/BuildingEditor/Core/Inputs/IA/IA_Turn.IA_Turn"))
  (Class|BuildingPawn|Turn ActionValue))

(event Input|EnhancedActionEvents|EnhancedInputActionIA_Zoom
  (params (ActionValue :type Float%20%28double-precision%29) (ElapsedSeconds :type Float%20%28double-precision%29) (TriggeredSeconds :type Float%20%28double-precision%29) (InputAction :type Input%20Action%20Object%20Reference :default "/Game/BuildingEditor/Core/Inputs/IA/IA_Zoom.IA_Zoom"))
  (bind _newtrack_0 (Timeline|ScrollTimeline PlayFromStart)
    (:Update
      (Class|BuildingPawn|Zoom (* _newtrack_0 ActionValue)))))

(event Input|EnhancedActionEvents|EnhancedInputActionIA_ToggleRotate
  (params (ActionValue :type Boolean) (ElapsedSeconds :type Float%20%28double-precision%29) (TriggeredSeconds :type Float%20%28double-precision%29) (InputAction :type Input%20Action%20Object%20Reference :default "/Game/BuildingEditor/Core/Inputs/IA/IA_ToggleRotate.IA_ToggleRotate"))
  (bind _cursorwidget (Variables|Default|GetCursorWidget))
  (:Triggered
    (Variables|/Game/BuildingEditor/Core/Character/Widgets/WBP_Cursor.WBP_Cursor_C|SetCursorIcon _cursorwidget (Variables|BuildingPawn|CursorIcons|GetRotateCursor)))
  (:Canceled
    (Variables|/Game/BuildingEditor/Core/Character/Widgets/WBP_Cursor.WBP_Cursor_C|SetCursorIcon _cursorwidget (Variables|BuildingPawn|CursorIcons|GetDefaultCursor) :!label _label))
  (:Completed
    (goto _label)))

(event Input|EnhancedActionEvents|EnhancedInputActionIA_ToggleTranslate
  (params (ActionValue :type Boolean) (ElapsedSeconds :type Float%20%28double-precision%29) (TriggeredSeconds :type Float%20%28double-precision%29) (InputAction :type Input%20Action%20Object%20Reference :default "/Game/BuildingEditor/Core/Inputs/IA/IA_ToggleTranslate.IA_ToggleTranslate"))
  (bind _cursorwidget (Variables|Default|GetCursorWidget))
  (:Triggered
    (Variables|/Game/BuildingEditor/Core/Character/Widgets/WBP_Cursor.WBP_Cursor_C|SetCursorIcon _cursorwidget (Variables|BuildingPawn|CursorIcons|GetMoveCursor)))
  (:Canceled
    (Variables|/Game/BuildingEditor/Core/Character/Widgets/WBP_Cursor.WBP_Cursor_C|SetCursorIcon _cursorwidget (Variables|BuildingPawn|CursorIcons|GetDefaultCursor) :!label _label))
  (:Completed
    (goto _label)))

(fn ConstructionScript)

(fn SnaptoGrid
  (params (Location :type Vector) (SnapValue :type Integer))
  (bind _returnvalue (/ Location SnapValue))
  (return (* (Math|Vector|MakeVector (Math|Conversions|ToFloat(Integer) (Math|Float|Round (.x _returnvalue))) (Math|Conversions|ToFloat(Integer) (Math|Float|Round (.y _returnvalue))) (Math|Conversions|ToFloat(Integer) (Math|Float|Round (.z _returnvalue)))) SnapValue)))